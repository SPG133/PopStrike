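; Player controller for PopStrike that registers Enhanced Input mapping contexts for the local player.
; On BeginPlay it adds a base context, then a higher-priority match context, and binds to possessed-pawn changes.
; When the new pawn implements BPI_AnimationBlueprintInterface, it adds the context and priority that pawn returns through GetIMCMessage.
; Contexts from previously possessed pawns are not removed.
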(event `self.ReceiveBeginPlay`
  (`self.SetUpBaseInputSystem`)
  (if (`self.IsLocalController`)
    (`EnhancedInputSubsystemInterface.AddMappingContext` (subsystem `EnhancedInputLocalPlayerSubsystem`) "/Game/PopStrike/Input/IMC_Match.IMC_Match" 1 (struct))
    (add `self.OnPossessedPawnChanged` (delegate `HandlePossessedPawnChangedEvent`))))

(event `HandlePossessedPawnChangedEvent` :!signature `self.OnPossessedPawnChanged`
  (params (OldPawn :type "Pawn Object Reference") (NewPawn :type "Pawn Object Reference"))
  (`self.HandlePossessedPawnChanged` OldPawn NewPawn))

(fn `HandlePossessedPawnChanged`
  (params (`Old Pawn` :type "Pawn Object Reference") (`New Pawn` :type "Pawn Object Reference"))
  (`/Engine/EditorBlueprintResources/StandardMacros.IsValid` (`local.New Pawn`)
    (:`Is Valid`
      (if (`KismetSystemLibrary.DoesImplementInterface` (`local.New Pawn`) "/Game/PopStrike/Interfaces/BPI_AnimationBlueprintInterface.BPI_AnimationBlueprintInterface_C")
        (bind (_imc _priority) (message `/Game/PopStrike/Interfaces/BPI_ChangeIMC.GetIMC` (`local.New Pawn`)))
        (`EnhancedInputSubsystemInterface.AddMappingContext` (subsystem `EnhancedInputLocalPlayerSubsystem`) _imc _priority (struct))))))

(fn `SetUpBaseInputSystem`
  (if (`self.IsLocalController`)
    (`EnhancedInputSubsystemInterface.AddMappingContext` (subsystem `EnhancedInputLocalPlayerSubsystem`) "/Game/PopStrike/Input/IMC_Base.IMC_Base" 0 (struct))))

(fn `UserConstructionScript`)