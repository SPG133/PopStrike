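; Player character for PopStrike, handling Enhanced Input look, movement, aiming and weapon switching.
; Weapon switching records the equipped gun and links the matching rifle, pistol or unarmed anim class layers on the mesh.
; Aim press and release switch the gate via UpdateGate, which informs the AnimInstance and applies speed, acceleration and braking from the GateSettings map.
; The equipped-gun message to the AnimInstance is unwired and never runs.
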(event `self.ReceiveBeginPlay`
  ;[0.02505 0.15 0.08238 0.5] Get EnhancedInputSystem
  (bind _asplayer_controller (cast `PlayerController` (`self.GetController`)))
  (`EnhancedInputSubsystemInterface.AddMappingContext` (pcsubsystem `EnhancedInputLocalPlayerSubsystem` _asplayer_controller) "/Game/PopStrike/Input/IMC_Match.IMC_Match" 0 (struct))
  ;[0.02505 0.15 0.08238 0.5] Set Default Idle
  (`SkeletalMeshComponent.LinkAnimClassLayers` (`self.Mesh`) "/Game/PopStrike/Animations/ABP_UnArmed.ABP_UnArmed_C"))

(event `EnhancedInput|/Game/PopStrike/Input/IA_SwitchWeapon`
  (params (ActionValue :type "Float (double-precision)") (ElapsedSeconds :type "Float (double-precision)") (TriggeredSeconds :type "Float (double-precision)") (InputAction :type "InputAction Object Reference" :default "/Game/PopStrike/Input/IA_SwitchWeapon.IA_SwitchWeapon"))
  (bind _mesh (`self.Mesh`))
  ;[1 0.3467 0.01161] Change Weapon
  (:`Started`
    (switch `int` (`KismetMathLibrary.FTrunc` ActionValue)
      (:`1`
        (set `self.EquipedGun` "NewEnumerator2")
        ;[0 0.6585 1] Change Weapon AnimLayers
        (`SkeletalMeshComponent.LinkAnimClassLayers` _mesh "/Game/PopStrike/Animations/ABP_Rifle.ABP_Rifle_C"))
      (:`2`
        (set `self.EquipedGun` "NewEnumerator1")
        (`SkeletalMeshComponent.LinkAnimClassLayers` _mesh "/Game/PopStrike/Animations/ABP_Pistol.ABP_Pistol_C"))
      (:`3`
        (set `self.EquipedGun` "NewEnumerator0")
        (`SkeletalMeshComponent.LinkAnimClassLayers` _mesh "/Game/PopStrike/Animations/ABP_UnArmed.ABP_UnArmed_C")))))

(event `EnhancedInput|/Game/PopStrike/Input/IA_Look`
  (params (ActionValue :type "Vector2D Structure") (ElapsedSeconds :type "Float (double-precision)") (TriggeredSeconds :type "Float (double-precision)") (InputAction :type "InputAction Object Reference" :default "/Game/PopStrike/Input/IA_Look.IA_Look"))
  (bind (_x _y) (`KismetMathLibrary.BreakVector2D` ActionValue))
  ;[1 0.3467 0.01161] LookAround
  (:`Triggered`
    (`self.AddControllerYawInput` _x)
    (`self.AddControllerPitchInput` _y)))

(event `EnhancedInput|/Game/PopStrike/Input/IA_Aim`
  (params (ActionValue :type Boolean) (ElapsedSeconds :type "Float (double-precision)") (TriggeredSeconds :type "Float (double-precision)") (InputAction :type "InputAction Object Reference" :default "/Game/PopStrike/Input/IA_Aim.IA_Aim"))
  ;[1 0.3467 0.01161] Aim
  (:`Started`
    (`self.UpdateGate` "NewEnumerator0"))
  (:`Completed`
    (`self.UpdateGate` "NewEnumerator1")))

(event `EnhancedInput|/Game/PopStrike/Input/IA_Move`
  (params (ActionValue :type "Vector2D Structure") (ElapsedSeconds :type "Float (double-precision)") (TriggeredSeconds :type "Float (double-precision)") (InputAction :type "InputAction Object Reference" :default "/Game/PopStrike/Input/IA_Move.IA_Move"))
  (bind (_x _y) (`KismetMathLibrary.BreakVector2D` ActionValue))
  (bind (_returnvalue_roll _returnvalue_pitch _returnvalue_yaw) (`KismetMathLibrary.BreakRotator` (`self.GetControlRotation`)))
  (bind (_returnvalue_roll_2 _returnvalue_pitch_2 _returnvalue_yaw_2) (`KismetMathLibrary.BreakRotator` (`self.GetControlRotation`)))
  ;[1 0.3467 0.01161] MoveForwardAndBackward
  (:`Triggered`
    (`self.AddMovementInput` (`KismetMathLibrary.GetRightVector` (`KismetMathLibrary.MakeRotator` _returnvalue_roll_2 0.0 _returnvalue_yaw_2)) _x)
    (`self.AddMovementInput` (`KismetMathLibrary.GetForwardVector` (`KismetMathLibrary.MakeRotator` 0.0 0.0 _returnvalue_yaw)) _y)))

(fn `UpdateGate`
  (params (Gate :type "/Game/PopStrike/Enums/E_Gate Enum" :default "NewEnumerator0"))
  (bind _charactermovement (`self.CharacterMovement`))
  (bind (_maxwalkspeed _maxacceleration _brakingdeceleration _brakingfrictionfactor _brakingfriction _useseperatebrakingfriction) (break `/Game/PopStrike/Struct/S_GateSetting` (`BlueprintMapLibrary.Map_Find` (`self.GateSettings`) (`local.Gate`))))
  (set `self.CurrentGate` Gate)
  ;[1 0.3698 0.9633] InformAnim
  (message `/Game/PopStrike/Interfaces/BPI_AnimationBlueprintInterface.ReceiveCurrentGate` (`SkeletalMeshComponent.GetAnimInstance` (`self.Mesh`)) Gate)
  (`|ExecutionSequence`
    (:`then_0`
      (set `CharacterMovementComponent.MaxWalkSpeed` _maxwalkspeed _charactermovement))
    (:`then_1`
      (set `CharacterMovementComponent.MaxAcceleration` _maxacceleration _charactermovement))
    (:`then_2`
      (set `CharacterMovementComponent.BrakingDecelerationWalking` _brakingdeceleration _charactermovement))
    (:`then_3`
      (set `CharacterMovementComponent.BrakingFrictionFactor` _brakingfrictionfactor _charactermovement))
    (:`then_4`
      (set `CharacterMovementComponent.BrakingFriction` _brakingfriction _charactermovement))
    (:`then_5`
      (set `CharacterMovementComponent.bUseSeparateBrakingFriction` _useseperatebrakingfriction _charactermovement))))

(fn `UserConstructionScript`)