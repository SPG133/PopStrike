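; PopStrike character Blueprint handling input for moving, looking, jumping, crouching and quiet slow walking, with movement input applied only on the ground.
; Crouch and slow-walk changes message the AnimInstance and re-run DecideGait, which sets max walk speed from GaitDict by slow-walk state alone.
; Linked anim layers start unarmed and switch to rifle for primary weapons.
; It also applies two-color dynamic materials and plays footstep-component sounds on hard landings.
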(event `self.OnLanded`
  (params (Hit :type "HitResult Structure (by ref)"))
  (bind _returnvalue (`KismetMathLibrary.Abs` (.z (`self.GetVelocity`))))
  ;[0.15 0.8348 0.15 0.5] PlayJumpSound
  (if (not (< _returnvalue (`self.FallDownVelocityThreshold`)))
    (message `/Game/PopStrike/Interfaces/BPI_SoundPlayer.PlayJumpSound` (`self.BP_FootstepComponent`) "NewEnumerator1" _returnvalue)))

(event `self.OnAppearanceChanged`
  (params (PrimaryColor :type "LinearColor Structure") (SecondaryColor :type "LinearColor Structure"))
  ;[0.15 0.8348 0.15 0.5] SetMaterial
  (bind _returnvalue (`PrimitiveComponent.CreateDynamicMaterialInstance` (`self.Mesh`) 0 null "PrimaryColor"))
  (`MaterialInstanceDynamic.SetVectorParameterValue` _returnvalue "None" PrimaryColor)
  (bind _returnvalue_2 (`PrimitiveComponent.CreateDynamicMaterialInstance` (`self.Mesh`) 1 null "SecondaryColor"))
  (`MaterialInstanceDynamic.SetVectorParameterValue` _returnvalue_2 "None" SecondaryColor))

(event `EnhancedInput|/Game/PopStrike/Input/IA_Crouch`
  (params (ActionValue :type Boolean) (ElapsedSeconds :type "Float (double-precision)") (TriggeredSeconds :type "Float (double-precision)") (InputAction :type "InputAction Object Reference" :default "/Game/PopStrike/Input/IA_Crouch.IA_Crouch"))
  ;[1 0.3467 0.01161] Input&Event_Crouch
  (:`Started`
    (`self.Crouch`))
  (:`Completed`
    (`self.UnCrouch`)))

(event `EnhancedInput|/Game/PopStrike/Input/IA_Quiet`
  (params (ActionValue :type Boolean) (ElapsedSeconds :type "Float (double-precision)") (TriggeredSeconds :type "Float (double-precision)") (InputAction :type "InputAction Object Reference" :default "/Game/PopStrike/Input/IA_Quiet.IA_Quiet"))
  ;[1 0.3467 0.01161] Input&Event_QuietSlow
  (:`Started`
    (`self.SetIsSlowWalking` true))
  (:`Completed`
    (`self.SetIsSlowWalking` false)))

(event `self.OnIsCrouchingChanged`
  (params (bNewValue :type Boolean))
  ;[1 0.3467 0.01161] Input&Event_Crouch
  (message `/Game/PopStrike/Interfaces/BPI_AnimationBlueprintInterface.ReceiveCrouching` (`SkeletalMeshComponent.GetAnimInstance` (`self.Mesh`)) bNewValue)
  (`self.DecideGait`))

(event `self.OnIsSlowWalkingChanged`
  (params (bNewValue :type Boolean))
  ;[1 0.3467 0.01161] Input&Event_QuietSlow
  (message `/Game/PopStrike/Interfaces/BPI_AnimationBlueprintInterface.ReceiveQuiet` (`SkeletalMeshComponent.GetAnimInstance` (`self.Mesh`)) bNewValue)
  (`self.DecideGait`))

(event `EnhancedInput|/Game/PopStrike/Input/IA_Move`
  (params (ActionValue :type "Vector2D Structure") (ElapsedSeconds :type "Float (double-precision)") (TriggeredSeconds :type "Float (double-precision)") (InputAction :type "InputAction Object Reference" :default "/Game/PopStrike/Input/IA_Move.IA_Move"))
  (bind (_returnvalue_roll _returnvalue_pitch _returnvalue_yaw) (`KismetMathLibrary.BreakRotator` (`self.GetControlRotation`)))
  (bind (_x _y) (`KismetMathLibrary.BreakVector2D` ActionValue))
  ;[1 0.3467 0.01161] Input_Move
  (:`Triggered`
    (if (`NavMovementComponent.IsMovingOnGround` (`self.CharacterMovement`))
      (`self.AddMovementInput` (`KismetMathLibrary.GetRightVector` (`KismetMathLibrary.MakeRotator` _returnvalue_roll 0.0 _returnvalue_yaw)) _x)
      (`self.AddMovementInput` (`KismetMathLibrary.GetForwardVector` (`KismetMathLibrary.MakeRotator` 0.0 0.0 _returnvalue_yaw)) _y))))

(event `EnhancedInput|/Game/PopStrike/Input/IA_Look`
  (params (ActionValue :type "Vector2D Structure") (ElapsedSeconds :type "Float (double-precision)") (TriggeredSeconds :type "Float (double-precision)") (InputAction :type "InputAction Object Reference" :default "/Game/PopStrike/Input/IA_Look.IA_Look"))
  (bind (_x _y) (`KismetMathLibrary.BreakVector2D` ActionValue))
  ;[1 0.3467 0.01161] Input_Look
  (:`Triggered`
    (`self.AddControllerYawInput` _x)
    (`self.AddControllerPitchInput` _y)))

(event `self.ReceiveBeginPlay`
  ;[1 0.06125 0.09084] BeginPlay
  (`SkeletalMeshComponent.LinkAnimClassLayers` (`self.Mesh`) "/Game/PopStrike/Animations/ABP_Unarmed.ABP_Unarmed_C")
  (`self.DecideGait`))

(event `EnhancedInput|/Game/PopStrike/Input/IA_Jump`
  (params (ActionValue :type Boolean) (ElapsedSeconds :type "Float (double-precision)") (TriggeredSeconds :type "Float (double-precision)") (InputAction :type "InputAction Object Reference" :default "/Game/PopStrike/Input/IA_Jump.IA_Jump"))
  ;[1 0.3467 0.01161] Input_Jump
  (:`Started`
    (`self.Jump`))
  (:`Completed`
    (`self.StopJumping`)))

(fn `DecideGait`
  (bind _gaitdict (`self.GaitDict`))
  (if (`self.IsSlowWalking`)
    (`self.SetGait` (`BlueprintMapLibrary.Map_Find` _gaitdict "quietslow_unarmed"))
    (else
      (`self.SetGait` (`BlueprintMapLibrary.Map_Find` _gaitdict "walk_unarmed")))))

(fn `EquipWeapon`
  (params (Weapon :type "PSWeaponBase Object Reference"))
  (`KismetSystemLibrary.PrintString` (`KismetSystemLibrary.GetDisplayName` Weapon))
  (`/Engine/EditorBlueprintResources/StandardMacros.IsValid` Weapon
    (:`Is Valid`
      (switch `EPSWeaponSlot` (`PSWeaponBase.WeaponSlot` (`local.Weapon`))
        (:`Primary`
          (`SkeletalMeshComponent.LinkAnimClassLayers` (`self.Mesh`) "/Game/PopStrike/Animations/ABP_Rifle.ABP_Rifle_C"))))))

(fn `SetGait`
  (params (Gait :type "/Game/PopStrike/Struct/S_GateSetting Structure"))
  (set `CharacterMovementComponent.MaxWalkSpeed` (`.MaxWalkSpeed_4_10DAE083465701ECAE7FA59052EB3D2B` (break `/Game/PopStrike/Struct/S_GateSetting` Gait)) (`self.CharacterMovement`)))

(fn `UserConstructionScript`)