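; BP_FootstepComponent is an actor component that plays footstep and landing sounds for its BP_Character owner in PopStrike.
; On BeginPlay it caches the character and its Sound data.
; PlayFootPrint skips playback while the character is slow walking, while PlayJumpSound always plays.
; Both call PlayFootstep, which selects the FootStep or Down sound by SoundKind and plays it at the owner's location.
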(event `self.ReceiveBeginPlay`
  (bind _asbp_character (cast `/Game/PopStrike/Blueprints/BP_Character` (`self.GetOwner`)))
  (set `self.OwnCharacter` _asbp_character)
  (set `self.Sound` (`/Game/PopStrike/Blueprints/BP_Character.Sound` _asbp_character)))

(event `/Game/PopStrike/Interfaces/BPI_SoundPlayer.PlayFootPrint`
  (params (SoundKind :type "/Game/PopStrike/Enums/E_SoundKind Enum" :default "NewEnumerator0"))
  (if (not (`PSFPSCharacter.IsSlowWalking` (`self.OwnCharacter`)))
    (`self.PlayFootstep` SoundKind (`Actor.K2_GetActorLocation` (`self.GetOwner`)))))

(event `/Game/PopStrike/Interfaces/BPI_SoundPlayer.PlayJumpSound`
  (params (SoundKind :type "/Game/PopStrike/Enums/E_SoundKind Enum" :default "NewEnumerator0") (Z_Velocity :type "Float (double-precision)"))
  (`self.PlayFootstep` SoundKind (`Actor.K2_GetActorLocation` (`self.GetOwner`))))

(fn `PlayFootstep`
  (params (SoundKind :type "/Game/PopStrike/Enums/E_SoundKind Enum" :default "NewEnumerator0") (Position :type "Vector Structure") (SoundRate :type "Float (double-precision)" :default 1.0))
  (bind (_footstep _down) (break `/Game/PopStrike/Struct/S_Sound` (`self.Sound`)))
  (`GameplayStatics.PlaySoundAtLocation` (select `/Game/PopStrike/Enums/E_SoundKind` SoundKind :`NewEnumerator0` _footstep :`NewEnumerator1` _down) Position (struct) SoundRate 1.0 0.0 null null null null))